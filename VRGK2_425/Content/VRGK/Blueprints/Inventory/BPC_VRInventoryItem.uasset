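; BPC_VRInventoryItem is an actor component that lets its owning actor be stored in and dropped from a VR inventory slot.
; Storing disables physics and collision, optionally hides the owner, and attaches it to the slot with a relative offset and fixed or hand-based rotation.
; Dropping detaches it and restores physics, collision and visibility.
; The slot reference tracks stored state, and both operations broadcast an inventory update.
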(event `Store In Inventory Slot`
  (params (InventorySlot :type "/Game/VRGK/Blueprints/Inventory/BP_VRInventorySlot_Base Object Reference"))
  (bind _returnvalue (`self.GetOwner`))
  ;[1 1 1] Store Item in Inventory Slot
  (set `self.InventorySlot` InventorySlot)
  (`PrimitiveComponent.SetSimulatePhysics` (`self.Get Root Primitive Component`) false)
  (`Actor.SetActorEnableCollision` _returnvalue false)
  (`Actor.SetActorHiddenInGame` _returnvalue (`self.HideInInventory`))
  (`Actor.K2_AttachToActor` _returnvalue (`self.InventorySlot`) "None" "SnapToTarget" (select `/Game/VRGK/Blueprints/Inventory/Enum_InventoryRotationRule` (`self.RotationRule`) :`NewEnumerator0` "SnapToTarget" :`NewEnumerator2` "KeepWorld" :!type "EAttachmentRule Enum") "KeepRelative" false)
  (`|ExecutionSequence`
    (:`then_0`
      (`Actor.K2_SetActorRelativeLocation` (`self.GetOwner`) (`self.RelativeLocation`) false false)
      (switch `/Game/VRGK/Blueprints/Inventory/Enum_InventoryRotationRule` (`self.RotationRule`)
        (:`NewEnumerator0`
          (`Actor.K2_SetActorRelativeRotation` (`self.GetOwner`) (`self.RelativeRotation`) false false))))
    (:`then_1`
      (`self.OnInventoryItemUpdate` true))))

(event `Drop  From Inventory Slot`
  (bind _returnvalue (`self.GetOwner`))
  ;[1 1 1] Drop Item from Inventory Slot
  (`self.InventorySlot`
    (:`then`
      (`|ExecutionSequence`
        (:`then_0`
          (`Actor.SetActorEnableCollision` _returnvalue true)
          (`Actor.SetActorHiddenInGame` _returnvalue false)
          (`Actor.K2_DetachFromActor` _returnvalue "KeepWorld" "KeepWorld" "KeepWorld")
          (`PrimitiveComponent.SetSimulatePhysics` (`self.Get Root Primitive Component`) true))
        (:`then_1`
          (set `self.InventorySlot` null)
          (`self.OnInventoryItemUpdate` false))))
    (:`else`)))

(fn `CanBeStored`
  (returns (True :type Boolean))
  (`/Engine/EditorBlueprintResources/StandardMacros.IsValid` (`self.InventorySlot`)
    (:`Is Valid`
      (return false))
    (:`Is Not Valid`
      (return true))))

(fn `Get Root Primitive Component`
  (returns (`AsPrimitive Component` :type "PrimitiveComponent Object Reference") (bSuccess :type Boolean))
  (bind (_asprimitive_component _bsuccess) (cast `PrimitiveComponent` (`Actor.RootComponent` (`self.GetOwner`)) :!pure true))
  (return _asprimitive_component _bsuccess))

(fn `Is in Inventory`
  (returns (True :type Boolean))
  (return (`KismetSystemLibrary.IsValid` (`self.InventorySlot`))))