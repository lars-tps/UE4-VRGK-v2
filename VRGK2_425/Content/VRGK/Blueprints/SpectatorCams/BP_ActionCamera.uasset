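; BP_ActionCamera is a spectator camera actor that follows the player's view with smoothed rotation.
; On BeginPlay it sets its spring arm to tick post-physics, including while paused, then snaps and attaches itself to the player camera manager.
; Rotation lag is switched on after a zero-length delay following the attach, so smoothing begins once the actor is in place.
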(event `self.ReceiveBeginPlay`
  (bind _springarm (`self.SpringArm`))
  (bind _springarm_2 (`self.SpringArm`))
  (`ActorComponent.SetTickGroup` _springarm_2 "TG_PostPhysics")
  (`ActorComponent.SetTickableWhenPaused` _springarm_2 true)
  (`KismetSystemLibrary.Delay` 0.0)
  (`self.K2_AttachToActor` self (`GameplayStatics.GetPlayerCameraManager` 0) "None" "SnapToTarget" "SnapToTarget" "SnapToTarget" true)
  (`KismetSystemLibrary.Delay` 0.0)
  (set `SpringArmComponent.CameraRotationLagSpeed` 5.0 _springarm)
  (set `SpringArmComponent.bEnableCameraRotationLag` true _springarm))

(fn `UserConstructionScript`)