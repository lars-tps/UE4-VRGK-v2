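; BPC_HingeSound is a component that plays a sound when a hinged physics component rotates, such as on a VR prop.
; Each tool tick it compares the physics component's rotation, measured in root component space, with the last sample.
; When the summed per-axis change exceeds a threshold, it spawns an attached sound with volume scaled by the excess.
; A DoOnce reset after a delay limits overlapping sounds.
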(event `self.Setup`
  (params (RootCompenent :type "SceneComponent Object Reference") (PhysicsComponent :type "PrimitiveComponent Object Reference"))
  (`parent.Setup` RootCompenent PhysicsComponent)
  (set `self.LastRotation` (`self.GetHingeRotation`)))

(event `self.UpdateToolTick`
  (params (DeltaSeconds :type "Float (single-precision)"))
  (bind _rotator (`self.GetHingeRotation`))
  (bind (_returnvalue_roll _returnvalue_pitch _returnvalue_yaw) (`KismetMathLibrary.BreakRotator` (`KismetMathLibrary.NormalizedDeltaRotator` _rotator (`self.LastRotation`))))
  (bind _returnvalue (+ (`KismetMathLibrary.Abs` _returnvalue_roll) (`KismetMathLibrary.Abs` _returnvalue_pitch) (`KismetMathLibrary.Abs` _returnvalue_yaw)))
  (`parent.UpdateToolTick` 0.0)
  (if (> _returnvalue (`self.RotationThreshold`))
    (`|ExecutionSequence`
      (:`then_0`
        (`/Engine/EditorBlueprintResources/StandardMacros.DoOnce` false :!label _label
          (:`Completed`
            (`GameplayStatics.SpawnSoundAttached` (`self.HingeSound`) (`self.RootComponent`) "None" (0.0 0.0 0.0) (struct) "KeepRelativeOffset" false (`KismetMathLibrary.FClamp` (/ (- _returnvalue (`self.RotationThreshold`)) (`self.RotationRange`))) 1.0 0.0 null null)
            ;[1 1 1] Reset after Delay
            (`KismetSystemLibrary.Delay` (`self.SoundOverlapDelay`))
            (goto _label :!via `Reset`))))
      (:`then_1`
        _)))
  (set `self.LastRotation` _rotator))

(fn `GetHingeRotation`
  (returns (Rotator :type "Rotator Structure"))
  (return (`KismetMathLibrary.InverseTransformRotation` (`SceneComponent.K2_GetComponentToWorld` (`self.RootComponent`)) (`SceneComponent.K2_GetComponentRotation` (`self.PhysicsComponent`)))))