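; Actor component that tracks which VR hands hold its owner and updates the owner's collision to match.
; Registering or unregistering a hand optionally swaps the root static mesh between grab and default collision profiles, then broadcasts OnCollisionUpdate.
; While held, it can bind to owner hit events, using a short retriggerable delay to keep a colliding flag set.
; IsColliding returns that flag, which the owner can force true through an interface.
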(event `UpdateHitEvents`
  (bind _returnvalue (`self.GetOwner`))
  (bind _actorhitisbound (`self.ActorHitIsBound`))
  ;[0.651 0.2594 0] Collision Hits. Useful for PD Checks on Hands.
  ; !!! Primitive Components of Owner need "Generate Hit Events" enabled !!!
  (if (`self.RegisterCollisionHitEvents`)
    (if (`self.HasHandAttached`)
      (if (not _actorhitisbound)
        (add `Actor.OnActorHit` _returnvalue (delegate `OnOwnerHit`))
        (set `self.ActorHitIsBound` true))
      (elif _actorhitisbound
        (remove `Actor.OnActorHit` _returnvalue (delegate `OnOwnerHit`))
        (set `self.ActorHitIsBound` false)))))

(event `RegisterHand`
  (params (VRHand :type "/Game/VRGK/Blueprints/Player/Hand/BP_VRHand Object Reference"))
  ;[1 1 1] Register Hand,  Hand has grabbed this Object.
  (if (not (`KismetArrayLibrary.Array_Contains` (`self.GrabHandArray`) VRHand))
    (`KismetArrayLibrary.Array_AddUnique` (`self.GrabHandArray`) VRHand)
    (`self.UpdateCollisionProfileState`)
    (`self.UpdateHitEvents`)))

(event `UnregisterHand`
  (params (VRHand :type "/Game/VRGK/Blueprints/Player/Hand/BP_VRHand Object Reference"))
  ;[1 1 1] Unregister Hand, Hand has dropped this Object.
  (if (`KismetArrayLibrary.Array_Contains` (`self.GrabHandArray`) VRHand)
    (`KismetArrayLibrary.Array_RemoveItem` (`self.GrabHandArray`) VRHand)
    (`self.UpdateCollisionProfileState`)
    (`self.UpdateHitEvents`)))

(event `OnOwnerHit`
  (params (SelfActor :type "Actor Object Reference") (OtherActor :type "Actor Object Reference") (NormalImpulse :type "Vector Structure") (Hit :type "HitResult Structure (by ref)"))
  ;[0.651 0.2594 0] Collision Hits. Useful for PD Checks on Hands.
  ; !!! Primitive Components of Owner need "Generate Hit Events" enabled !!!
  (`|ExecutionSequence` :!label _label
    (:`then_0`
      (set `self.ObjectIsColliding` true))
    (:`then_1`
      (`KismetSystemLibrary.RetriggerableDelay` 0.1)
      (set `self.ObjectIsColliding` false))))

(event `OnHandCollisionHit`
  ;[0.651 0.2594 0] Collision Hits. Useful for PD Checks on Hands.
  ; !!! Primitive Components of Owner need "Generate Hit Events" enabled !!!
  (goto _label))

(event `UpdateCollisionProfileState`
  ;[0.7229 0.3022 1] Update Collision Profile State based on Grabbing or not Grabbing
  (if (`self.UpdateCollisionProfile`)
    (`|ExecutionSequence`
      (:`then_0`
        (bind _asstatic_mesh_component (cast `StaticMeshComponent` (`Actor.RootComponent` (`self.GetOwner`)))
          (:`then`
            (`PrimitiveComponent.SetCollisionProfileName` _asstatic_mesh_component (select `bool` (`self.HasHandAttached`) :`false` (`self.DefaultCollisionProfile`) :`true` (`self.GrabCollisionProfile`)) true))
          (:`CastFailed`
            ;;[1 0.4656 0.4656] Write a Message that there was an error
            (`KismetSystemLibrary.PrintString` "HandGrabCollisionUpdater can't find a Primitive Root Component."))))
      (:`then_1`
        (`self.OnCollisionUpdate` (`self.HasHandAttached`))))))

(fn `HasHandAttached`
  (returns (True :type Boolean))
  (return (> (`KismetArrayLibrary.Array_Length` (`self.GrabHandArray`)) 0)))

(fn `IsColliding`
  (returns (True :type Boolean))
  (if (`KismetSystemLibrary.DoesImplementInterface` (`self.GetOwner`) "/Game/VRGK/Blueprints/Components/GrabCollisionUpdater/BPI_HandGrabCollisionUpdater.BPI_HandGrabCollisionUpdater_C")
    (bind _is_colliding (message `/Game/VRGK/Blueprints/Components/GrabCollisionUpdater/BPI_HandGrabCollisionUpdater.IsForcingHitCollision` (`self.GetOwner`)))
    (return (or _is_colliding (`self.ObjectIsColliding`)))
    (else
      (return (`self.ObjectIsColliding`)))))