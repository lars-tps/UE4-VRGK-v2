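; Actor component that makes its owner destructible by physical impact.
; It binds to the owner's hit event and, when the impulse exceeds HitThreshold, plays a destruction sound and destroys the owner.
; An optional PartsActor spawns in its place, inheriting linear and angular velocity through BP_DestroyedActorBase's AddSpawnImpulse.
; A debug drawing event for hits exists but is disconnected.
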(event `self.ReceiveBeginPlay`
  (add `Actor.OnActorHit` (`self.GetOwner`) (delegate `OnActorHit`)))

(event `OnActorHit`
  (params (SelfActor :type "Actor Object Reference") (OtherActor :type "Actor Object Reference") (NormalImpulse :type "Vector Structure") (Hit :type "HitResult Structure (by ref)"))
  (bind _returnvalue (`self.GetOwner`))
  (bind (_returnvalue_location _returnvalue_rotation) (`KismetMathLibrary.BreakTransform` (`Actor.GetTransform` (`self.GetOwner`))))
  (if (!= SelfActor OtherActor)
    (`|ExecutionSequence`
      (:`then_0`
        (if (> (`KismetMathLibrary.VSize` NormalImpulse) (`self.HitThreshold`))
          (`|ExecutionSequence`
            (:`then_0`
              (`GameplayStatics.SpawnSoundAtLocation` (`self.DestructionSound`) (`.ImpactPoint` (`GameplayStatics.BreakHitResult` Hit)) (struct) 1.0 1.0 0.0 null null))
            (:`then_1`
              (`|ExecutionSequence`
                (:`then_0`
                  (if (`KismetSystemLibrary.IsValidClass` (`self.PartsActor`))
                    (bind _returnvalue_2 (`|SpawnActorFromClass` (`self.PartsActor`) (`KismetMathLibrary.MakeTransform` _returnvalue_location _returnvalue_rotation) "Undefined" "OverrideRootScale" null null))
                    (bind _asbp_destroyed_actor_base (cast `/Game/VRGK/Blueprints/Components/Destructible/BP_DestroyedActorBase` _returnvalue_2))
                    (bind _asprimitive_component (cast `PrimitiveComponent` (`Actor.RootComponent` _returnvalue))
                      (:`then`
                        (`/Game/VRGK/Blueprints/Components/Destructible/BP_DestroyedActorBase.AddSpawnImpulse` _asbp_destroyed_actor_base (`SceneComponent.GetComponentVelocity` _asprimitive_component) (`PrimitiveComponent.GetPhysicsAngularVelocityInDegrees` _asprimitive_component "None")))
                      (:`CastFailed`
                        (`/Game/VRGK/Blueprints/Components/Destructible/BP_DestroyedActorBase.AddSpawnImpulse` _asbp_destroyed_actor_base (`Actor.GetVelocity` _returnvalue) (0.0 0.0 0.0))))))
                (:`then_1`
                  (`Actor.K2_DestroyActor` (`self.GetOwner`)))))))))))

(event `DrawDebugHit`
  (params (NormalImpulse :type "Vector Structure") (Hit :type "HitResult Structure"))
  (bind (_bblockinghit _binitialoverlap _time _distance _location _impactpoint) (`GameplayStatics.BreakHitResult` Hit))
  (`KismetSystemLibrary.DrawDebugSphere` _impactpoint 10.0 4 (struct :`R` 1.0 :`B` 0.228938 :`A` 1.0) 0.2 1.0)
  (`KismetSystemLibrary.DrawDebugArrow` _impactpoint (+ _impactpoint (* NormalImpulse 0.01)) 5.0 (struct :`R` 1.0 :`G` 0.84287 :`A` 1.0) 0.2 1.0))