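; VR subtitle actor that shows text on a widget and lazily follows the player's view.
; It attaches to the camera manager, and Tick keeps the Scene component at the actor's location while subtitles are visible.
; A looping timer checks distance and rotation thresholds, then a DoOnce-gated timeline eases the Scene rotation toward the new view direction.
; Hiding pauses tick and timer, and the game's subtitle setting toggles the widget root.
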(event `OnSubtitleEnabledUpdate`
  (params (NewEnabled :type Boolean))
  ;[1 1 1] Begin Play Setup
  (bind _output_get (set `self.SubtitlesEnabled` NewEnabled))
  (`SceneComponent.SetHiddenInGame` (`self.WidgetRoot`) (not _output_get) true))

(event `self.ReceiveBeginPlay`
  ;[1 1 1] Begin Play Setup
  (`|ExecutionSequence`
    (:`then_0`
      (`self.CreateWidget`)
      (`self.K2_AttachToActor` self (`GameplayStatics.GetPlayerCameraManager` 0) "None" "SnapToTarget" "SnapToTarget" "KeepWorld" true))
    (:`then_1`
      (bind _returnvalue (`KismetSystemLibrary.K2_SetTimerDelegate` (delegate `UpdateTimer`) (`self.SubtitlePositionUpdateTime`) true))
      (set `self.TimerHandle` _returnvalue))
    (:`then_2`
      (`PrimitiveComponent.SetCastShadow` (`self.Widget`) false)
      (`self.SetSubtitleVisible` false)
      (bind _settings (`/Game/VRGK/Blueprints/BPFL_GlobalFunctions.Get BPO Game Settings`))
      (add `/Game/VRGK/Blueprints/Core/BPO_Settings.OnSubtitlesEnabled` _settings (delegate `OnSubtitleEnabledUpdate`))
      (`self.OnSubtitleEnabledUpdate` (`/Game/VRGK/Blueprints/Core/BPO_Settings.GetSubtitlesEnabled` _settings)))))

(event `CreateWidget`
  ;[1 1 1] Create Subtitle Widget
  (bind _returnvalue (`|CreateWidget` (`self.SubtitleWidgetClass`)))
  (bind _asbpw_vrsubtitles (cast `/Game/VRGK/Blueprints/Subtitles/BPW_VRSubtitles` _returnvalue))
  (set `self.SubtitleWidget` _asbpw_vrsubtitles)
  (`WidgetComponent.SetWidget` (`self.Widget`) (`self.SubtitleWidget`)))

(event `UpdateTimer`
  (bind (_newlocation _newrotation) (`self.GetNewPosition`))
  (bind (_transitionstarttransform_location _transitionstarttransform_rotation) (`KismetMathLibrary.BreakTransform` (`self.TransitionStartTransform`)))
  ;[1 1 1] Update Subtitle Position & Rotation
  (if (`self.NeedsMovementOfNewPosition` _newlocation _newrotation)
    (`/Engine/EditorBlueprintResources/StandardMacros.DoOnce` false :!label _label
      (:`Completed`
        (set `self.NewTargetLocation` _newlocation)
        (set `self.NewTargetRotation` _newrotation)
        (set `self.TransitionStartTransform` (`SceneComponent.K2_GetComponentToWorld` (`self.WidgetRoot`)))
        (bind (_direction _alpha) (`Timeline|PositionUpdateTimeline` :!via `PlayFromStart`)
          (:`Update`
            (`SceneComponent.K2_SetWorldRotation` (`self.Scene`) (`KismetMathLibrary.RLerp` _transitionstarttransform_rotation (`self.NewTargetRotation`) _alpha true) false false))
          (:`Finished`
            (goto _label :!via `Reset`)))))))

(event `self.ReceiveTick`
  (params (DeltaSeconds :type "Float (single-precision)"))
  ;[1 1 1] Event Tick and Position Updates
  (`self.UpdatePosition`))

(event `UpdatePosition`
  ;[1 1 1] Event Tick and Position Updates
  (`SceneComponent.K2_SetWorldLocation` (`self.Scene`) (`self.K2_GetActorLocation`) false false))

(event `ShowSubtitleWithText`
  (params (Text :type Text))
  ;[1 1 1] Show / Hide Subtitles
  (`self.SetSubtitleText` Text)
  (`self.SetSubtitleVisible` true))

(event `SetSubtitleText`
  (params (Text :type Text))
  ;[1 1 1] Set Subtitle Text
  (`/Game/VRGK/Blueprints/Subtitles/BPW_VRSubtitles.SetSubtitleText` (`self.SubtitleWidget`) Text))

(event `HideSubtitles`
  ;[1 1 1] Show / Hide Subtitles
  (`self.SetSubtitleVisible` false))

(event `SetSubtitleVisible`
  (params (Visible :type Boolean))
  ;[1 1 1] Set Subtitle Visibility
  (if Visible
    (`self.UpdatePosition`)
    (`self.SetActorTickEnabled` true)
    (`self.SetActorHiddenInGame` false)
    (`KismetSystemLibrary.K2_UnPauseTimerHandle` (`self.TimerHandle`))
    (else
      (`self.SetActorHiddenInGame` true)
      (`self.SetActorTickEnabled` false)
      (`KismetSystemLibrary.K2_PauseTimerHandle` (`self.TimerHandle`)))))

(fn `GetNewPosition`
  (returns (NewLocation :type "Vector Structure") (NewRotation :type "Rotator Structure"))
  (bind _returnvalue_location (`KismetMathLibrary.BreakTransform` (`self.GetTransform`)))
  (bind _returnvalue (`self.GetActorForwardVector`))
  (bind _returnvalue_2 (`KismetMathLibrary.Normal` (`KismetMathLibrary.ProjectVectorOnToPlane` _returnvalue (0.0 0.0 1.0))))
  (return (+ _returnvalue_location (* _returnvalue_2 80.0) (0.0 0.0 -25.0)) (`KismetMathLibrary.TransformRotation` (`KismetMathLibrary.MakeTransform` (0.0 0.0 0.0) (`KismetMathLibrary.FindLookAtRotation` (0.0 0.0 0.0) _returnvalue_2)) (`KismetMathLibrary.MakeRotator` 0.0 (* (.z _returnvalue) 60.0)))))

(fn `NeedsMovementOfNewPosition`
  (params (NewLocation :type "Vector Structure") (NewRotation :type "Rotator Structure"))
  (returns (True :type Boolean))
  (bind (_returnvalue_location _returnvalue_rotation) (`KismetMathLibrary.BreakTransform` (`SceneComponent.K2_GetComponentToWorld` (`self.WidgetRoot`))))
  (bind (_returnvalue_roll _returnvalue_pitch _returnvalue_yaw) (`KismetMathLibrary.BreakRotator` (`KismetMathLibrary.NormalizedDeltaRotator` NewRotation _returnvalue_rotation)))
  (return (or (> (`KismetMathLibrary.Vector_Distance` NewLocation _returnvalue_location) (`self.DistanceThreshold`)) (> (+ (`KismetMathLibrary.Abs` _returnvalue_roll) (`KismetMathLibrary.Abs` _returnvalue_pitch) (`KismetMathLibrary.Abs` _returnvalue_yaw)) (`self.RotationThreshold`)))))

(fn `UserConstructionScript`)