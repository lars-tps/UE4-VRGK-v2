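; VR character pawn that supports room-scale head movement alongside standard Character walking, sprinting and jumping.
; Each tick it measures the camera's horizontal offset from the actor, shifts VROriginRoot back and moves the capsule by the same amount, keeping the body under the headset.
; That capsule move is unswept, so it ignores blocking collision.
; Tick also sets walk speed from the sprint state, and the Jump input triggers a jump.
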(event `self.ReceiveBeginPlay`
  (`parent.ReceiveBeginPlay`))

(event `self.ReceiveTick`
  (params (DeltaSeconds :type "Float (single-precision)"))
  (`parent.ReceiveTick` DeltaSeconds)
  (`self.MovementUpdateTick` DeltaSeconds)
  (set `CharacterMovementComponent.MaxWalkSpeed` (`KismetMathLibrary.SelectFloat` 800.0 400.0 (`self.IsSprinting`)) (`self.CharacterMovement`)))

(event `MovementUpdateTick`
  (params (DeltaSeconds :type "Float (double-precision)"))
  ;[1 1 1] Movement Tick
  (`self.UpdateCameraBodyOffset`))

(event `UpdateCameraBodyOffset`
  (bind (_returnvalue_x _returnvalue_y) (`KismetMathLibrary.BreakVector` (* (`self.TempCameraOffset`) -1.0)))
  ;[1 1 1] Update Offset from Camera to Body.
  (set `self.TempCameraOffset` (`KismetMathLibrary.InverseTransformLocation` (`self.GetTransform`) (`SceneComponent.K2_GetComponentLocation` (`self.Camera`))))
  (`SceneComponent.K2_AddLocalOffset` (`self.VROriginRoot`) (`KismetMathLibrary.MakeVector` _returnvalue_x _returnvalue_y) false false)
  (`SceneComponent.K2_AddWorldOffset` (`self.CapsuleComponent`) (`KismetMathLibrary.TransformDirection` (`self.GetTransform`) (`KismetMathLibrary.MakeVector` (.x (* (`self.TempCameraOffset`) 1.0)) (.y (* (`self.TempCameraOffset`) 1.0)))) false false))

(event `InputAction|Jump`
  (params (Key :type "Key Structure"))
  (:`Pressed`
    (`self.Jump`)))

(fn `UserConstructionScript`
  (`parent.UserConstructionScript`))