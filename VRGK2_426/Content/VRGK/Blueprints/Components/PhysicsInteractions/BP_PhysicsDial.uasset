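; BP_PhysicsDial is a VR physics dial that turns the rotation of its physics component into a running value.
; On each tool update it takes the yaw delta of that component, measured relative to the root, since the last accepted rotation.
; When the delta exceeds a threshold, it adds it to the value, which can accumulate past a full turn, and calls the value-change notification.
; Getters expose the value and a yaw velocity derived from that delta.
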(event `self.ReceiveBeginPlay`
  (`parent.ReceiveBeginPlay`)
  (set `self.LastRotation` (`self.GetDialRotator`)))

(event `self.UpdateToolTick`
  (params (DeltaSeconds :type "Float (single-precision)"))
  (bind (_returnvalue_roll _returnvalue_pitch _returnvalue_yaw) (`KismetMathLibrary.BreakRotator` (`KismetMathLibrary.NormalizedDeltaRotator` (`self.TempRotation`) (`self.LastRotation`))))
  (`parent.UpdateToolTick` DeltaSeconds)
  (if (> DeltaSeconds 0.0)
    (set `self.TempRotation` (`self.GetDialRotator`))
    (set `self.TempValue` (+ (`self.CurrentValue`) _returnvalue_yaw))
    (set `self.DialVelocity` (`KismetMathLibrary.SelectFloat` 0.0 (* _returnvalue_yaw (/ 1.0 DeltaSeconds)) (== DeltaSeconds 0.0)))
    (if (> (`KismetMathLibrary.Abs` (- (`self.CurrentValue`) (`self.TempValue`))) (`self.AngleChangeThreshold`))
      (bind _output_get (set `self.CurrentValue` (`self.TempValue`)))
      (`self.OnValueChange` _output_get)
      (set `self.LastRotation` (`self.TempRotation`)))))

(fn `Get Current Dial Value`
  (returns (CurrentValue :type "Float (double-precision)"))
  (return (`self.CurrentValue`)))

(fn `GetCurrentDialVelocity`
  (returns (DialVelocity :type "Float (double-precision)"))
  (return (`self.DialVelocity`)))

(fn `GetDialRotator`
  (returns (ReturnValue :type "Rotator Structure"))
  (return (`KismetMathLibrary.InverseTransformRotation` (`SceneComponent.K2_GetComponentToWorld` (`self.RootComponent`)) (`SceneComponent.K2_GetComponentRotation` (`self.PhysicsComponent`)))))