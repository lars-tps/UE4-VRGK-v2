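; Blueprint function library in VRGK with helpers for physics objects in attachment hierarchies.
; AttachObjectToPhysicalParent enables simulation on a child actor's given root, then attaches it, keeping world transform, to the primitive its parent component hangs from, reporting that parent.
; GetPhysicsRoot climbs a movable, simulating component's parents and returns the last in the unbroken run of simulating primitives, if any.
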(fn `Attach Object to Physical Parent`
  (params (Actor :type "Actor Object Reference") (PrimRootComponent :type "PrimitiveComponent Object Reference"))
  (returns (NeedsReattach :type Boolean) (NewParentComponent :type "PrimitiveComponent Object Reference"))
  (bind _returnvalue (`Actor.GetParentComponent` Actor))
  (`/Engine/EditorBlueprintResources/StandardMacros.IsValid` _returnvalue
    (:`Is Valid`
      (bind _asprimitive_component (cast `PrimitiveComponent` (`SceneComponent.GetAttachParent` _returnvalue))
        (:`then`
          (`PrimitiveComponent.SetSimulatePhysics` (`local.PrimRootComponent`) true)
          (`SceneComponent.K2_AttachToComponent` (`local.PrimRootComponent`) _asprimitive_component "None" "KeepWorld" "KeepWorld" "KeepWorld" true)
          (return true _asprimitive_component))
        (:`CastFailed`
          (return false null))))
    (:`Is Not Valid`
      (return false null))))

(fn `GetPhysicsRoot`
  (params (Child :type "PrimitiveComponent Object Reference") (ChildBoneName :type Name))
  (returns (HasPhysicsRoot :type Boolean) (`Physics Root` :type "PrimitiveComponent Object Reference"))
  (locals (TempRoot :type "PrimitiveComponent Object Reference"))
  (switch `EComponentMobility` (`SceneComponent.Mobility` Child)
    (:`Static`
      _)
    (:`Stationary`
      _)
    (:`Movable`
      (if (`SceneComponent.IsSimulatingPhysics` (`local.Child`) (`local.ChildBoneName`))
        (for _array_element (`SceneComponent.GetParentComponents` (`local.Child`))
          (bind _asprimitive_component (cast `PrimitiveComponent` _array_element)
            (:`then`
              (if (`SceneComponent.IsSimulatingPhysics` _asprimitive_component "None")
                (set `local.TempRoot` _asprimitive_component)
                (else
                  (bind _temproot (`local.TempRoot` :!label _label)
                    (:`then`
                      (return true _temproot))
                    (:`else`
                      (return false null))))))
            (:`CastFailed`
              (goto _label))))
        (goto _label)
        (else
          (return false null)))))
  (return false null))