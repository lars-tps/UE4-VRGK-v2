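; VR player teleport arc actor that previews a teleport destination and reports whether it is valid.
; While enabled, it predicts a projectile path along its forward vector each tick, driving the Niagara arc's endpoint and color and a target marker.
; A hit is valid only within range, on a shallow enough slope, and where a body-sized sphere trace up to the pawn's current height is clear.
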(event `self.ReceiveBeginPlay`
  (`self.SetTeleportArcEnabled` false))

(event `self.ReceiveTick`
  (params (DeltaSeconds :type "Float (single-precision)"))
  (`self.UpdateArc`))

(event `UpdateArc`
  (bind _isvalidteleportlocation (`self.IsValidTeleportLocation`))
  (bind _targetlocationroot (`self.TargetLocationRoot`))
  ;[1 1 1] Update Arc and Trace Location for new Teleport Position
  (bind (_outhit _outpathpositions _outlasttracedestination _returnvalue) (`GameplayStatics.Blueprint_PredictProjectilePath_ByObjectType` (`self.K2_GetActorLocation`) (* (`self.GetActorForwardVector`) (`self.TeleportVelocity`)) true 0.0 (`self.TeleportObjectTypes`)))
  (bind (_valid _updatedfloorlocation) (`self.CheckForValidTeleportLocation` _outhit _outpathpositions _returnvalue))
  (set `self.IsValidTeleportLocation` _valid)
  (set `self.TeleportLocation` _updatedfloorlocation)
  (`|ExecutionSequence`
    (:`then_0`
      (if (!= (`SceneComponent.bVisible` _targetlocationroot) _isvalidteleportlocation)
        (`SceneComponent.SetVisibility` _targetlocationroot _isvalidteleportlocation true)
        (`self.UpdateArcColor` _isvalidteleportlocation)))
    (:`then_1`
      (if _valid
        (`FXSystemComponent.SetVectorParameter` (`self.NiagaraArc`) "EndLocation" _updatedfloorlocation)
        (`SceneComponent.K2_SetWorldLocation` (`self.TargetLocationRoot`) _updatedfloorlocation false false)
        (else
          (`FXSystemComponent.SetVectorParameter` (`self.NiagaraArc`) "EndLocation" _outlasttracedestination))))))

(event `UpdateArcColor`
  (params (Valid :type Boolean))
  ;[1 1 1] Update Arc Color
  (`FXSystemComponent.SetColorParameter` (`self.NiagaraArc`) "ArcColor" (`KismetMathLibrary.SelectColor` (struct :`R` 0.049707 :`G` 0.527115 :`B` 0.854993 :`A` 1.0) (struct :`R` 0.854993 :`G` 0.414332 :`B` 0.024622 :`A` 0.6) Valid)))

(event `SetTeleportArcEnabled`
  (params (Enabled :type Boolean))
  (bind _niagaraarc (`self.NiagaraArc`))
  ;[1 1 1] Enable / Disable Arc
  (if Enabled
    (`self.SetActorHiddenInGame` false)
    (`ActorComponent.Activate` _niagaraarc false)
    (`self.SetActorTickEnabled` true)
    (`SceneComponent.SetVisibility` (`self.TargetLocationRoot`) false true)
    (`self.UpdateArcColor` false)
    (`self.UpdateArc`)
    (else
      (`self.SetActorHiddenInGame` true)
      (`ActorComponent.Deactivate` _niagaraarc)
      (`self.SetActorTickEnabled` false)
      (set `self.IsValidTeleportLocation` false))))

(fn `CheckForValidTeleportLocation`
  (params (HitResult :type "HitResult Structure") (PathPositions :type "Array of Vector Structure") (Found :type Boolean))
  (returns (Valid :type Boolean) (UpdatedFloorLocation :type "Vector Structure"))
  (bind (_bblockinghit _binitialoverlap _time _distance _location _impactpoint _normal _impactnormal _physmat _hitactor _hitcomponent _hitbonename _hititem _faceindex _tracestart) (`GameplayStatics.BreakHitResult` (`local.HitResult`)))
  (bind _returnvalue (* (`self.BodyRadius`) 2.0))
  (bind _returnvalue_2 (+ (`.Location` (`GameplayStatics.BreakHitResult` (`local.HitResult`))) (`KismetMathLibrary.MakeVector` 0.0 0.0 _returnvalue)))
  (if Found
    ;[1 1 1] Check if the Teleport Location is a Slope
    (if (and (< (`KismetMathLibrary.Vector_Distance` (`self.K2_GetActorLocation`) _tracestart) (`self.MaxTeleportDistance`)) (> (`KismetMathLibrary.Dot_VectorVector` _normal (0.0 0.0 1.0)) (`self.SlopeThreshold`)))
      ;[1 1 1] Check if Player Body fits into the Teleport Location
      (bind (_outhit _returnvalue_3) (`KismetSystemLibrary.SphereTraceSingleForObjects` (+ _returnvalue_2 (`KismetMathLibrary.MakeVector` 0.0 0.0 (`KismetMathLibrary.SelectFloat` 10.0 0.0 (`|EnumEquality` (`PrimitiveComponent.GetCollisionObjectType` _hitcomponent) "ECC_GameTraceChannel6")))) (+ _returnvalue_2 (`KismetMathLibrary.MakeVector` 0.0 0.0 (- (`/Game/VRGK/Blueprints/Player/PlayerCore/BP_VRGamePawn.GetCurrentHeight` (`self.VRPawn`)) _returnvalue))) (`self.BodyRadius`) (`self.TeleportObjectTypes`)))
      (return (not _returnvalue_3) (`.Location` (`GameplayStatics.BreakHitResult` (`local.HitResult`))))
      (else
        (return false (0.0 0.0 0.0))))
    (else
      (return false (0.0 0.0 0.0)))))

(fn `GetTeleportLocation`
  (returns (Valid :type Boolean) (FloorLocation :type "Vector Structure"))
  (return (`self.IsValidTeleportLocation`) (`self.TeleportLocation`)))

(fn `UserConstructionScript`)