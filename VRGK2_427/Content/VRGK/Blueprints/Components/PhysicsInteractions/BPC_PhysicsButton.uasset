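; BPC_PhysicsButton is a VRGK physics interaction component that turns the movement of a physics component into a pressed or released button state.
; Each tool tick it compares the physics component's local Z, relative to the root, against separate press and release thresholds for hysteresis.
; An optional delay debounces state changes.
; Changes fire press or release events and play optional attached sounds, and a getter exposes the state.
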(event `self.ReceiveBeginPlay`
  ;[1 1 1] Setup
  (`parent.ReceiveBeginPlay`)
  (set `self.LastPressChange` (`KismetMathLibrary.Now`))
  (set `self.WatchForChangeDelay` (> (`self.PressChangeDelay`) 0.01)))

(event `self.UpdateToolTick`
  (params (DeltaSeconds :type "Float (single-precision)"))
  (bind _returnvalue (< (.z (`KismetMathLibrary.InverseTransformLocation` (`SceneComponent.K2_GetComponentToWorld` (`self.RootComponent`)) (`SceneComponent.K2_GetComponentLocation` (`self.PhysicsComponent`)))) (`KismetMathLibrary.SelectFloat` (`self.ReleaseZ`) (`self.PressZ`) (`self.Pressed`))))
  (if (`self.WatchForChangeDelay`)
    ;[1 1 1] Use Delay between Button Press State changes
    (bind _output_get (set `self.TempPressState` _returnvalue))
    (if (!= _output_get (`self.Pressed`))
      (if (>= (`KismetMathLibrary.Abs` (`KismetMathLibrary.GetTotalSeconds` (- (`self.LastPressChange`) (`KismetMathLibrary.Now`)))) (`self.PressChangeDelay`))
        (`self.SetButtonPressed` (`self.TempPressState`))
        (set `self.LastPressChange` (`KismetMathLibrary.Now`)))
      (else
        (set `self.LastPressChange` (`KismetMathLibrary.Now`))))
    (else
      (`self.SetButtonPressed` _returnvalue))))

(event `SetButtonPressed`
  (params (Pressed :type Boolean))
  (bind _presssound (`self.PressSound`))
  (bind _releasesound (`self.ReleaseSound`))
  ;[1 1 1] Set Button Pressed State
  (if (!= Pressed (`self.Pressed`))
    (bind _output_get (set `self.Pressed` Pressed))
    (if _output_get
      (`self.OnButtonPress`)
      (`/Engine/EditorBlueprintResources/StandardMacros.IsValid` _presssound
        (:`Is Valid`
          (`GameplayStatics.SpawnSoundAttached` _presssound (`self.RootComponent`) "None" (0.0 0.0 0.0) (struct) "KeepRelativeOffset" false 1.0 1.0 0.0 null null)))
      (else
        (`self.OnButtonRelease`)
        (`/Engine/EditorBlueprintResources/StandardMacros.IsValid` _releasesound
          (:`Is Valid`
            (`GameplayStatics.SpawnSoundAttached` _releasesound (`self.RootComponent`) "None" (0.0 0.0 0.0) (struct) "KeepRelativeOffset" false 1.0 1.0 0.0 null null)))))))

(fn `GetButtonPressedState`
  (returns (Pressed :type Boolean))
  (return (`self.Pressed`)))