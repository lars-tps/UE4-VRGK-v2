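; BPC_PhysicsSlider is a VRGK physics-interaction component that provides the value of a slider.
; GetToolValue converts the physics component's world location into the root component's local space and returns the X, Y or Z coordinate chosen by the Axis setting.
; The value is therefore a raw linear offset along that axis, with no normalization or clamping here.
; The event graph holds only disabled BeginPlay and Tick stubs.
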(fn `Get Tool Value`
  (returns (CurrentValue :type "Float (double-precision)"))
  (return (select `/Game/VRGK/Blueprints/Components/Enum_PhysicsToolAxis` (`self.Axis`) :`NewEnumerator0` (.x (`KismetMathLibrary.InverseTransformLocation` (`SceneComponent.K2_GetComponentToWorld` (`self.RootComponent`)) (`SceneComponent.K2_GetComponentLocation` (`self.PhysicsComponent`)))) :`NewEnumerator1` (.y (`KismetMathLibrary.InverseTransformLocation` (`SceneComponent.K2_GetComponentToWorld` (`self.RootComponent`)) (`SceneComponent.K2_GetComponentLocation` (`self.PhysicsComponent`)))) :`NewEnumerator2` (.z (`KismetMathLibrary.InverseTransformLocation` (`SceneComponent.K2_GetComponentToWorld` (`self.RootComponent`)) (`SceneComponent.K2_GetComponentLocation` (`self.PhysicsComponent`)))))))