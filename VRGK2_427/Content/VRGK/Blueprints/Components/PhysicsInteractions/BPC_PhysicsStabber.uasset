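; Physics tool component that lets an object stab into a hit component or bone and slide along the stab axis.
; SetupStabber configures the constraint with locked rotation and X/Y, limited Z and a velocity drive as friction, toggling simulation to apply disabled collision.
; After a short startup delay, tool ticks break the constraint once Z offset exceeds the limit.
; Destruction of the stabbed actor also breaks it, firing a broken callback.
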(event `self.ReceiveBeginPlay`
  ;[1 1 1] Begin Play and wait 0,3s before allowing to break stabber.
  (`parent.ReceiveBeginPlay`)
  (`KismetSystemLibrary.Delay` 0.3)
  (set `self.ActiveStabber` true))

(event `OnAttacherDestroyed`
  (params (DestroyedActor :type "Actor Object Reference"))
  ;[1 1 1] On stabbed Actor is destroyed
  (`self.DoBreakStabber`))

(event `self.UpdateToolTick`
  (params (DeltaSeconds :type "Float (single-precision)"))
  (bind _relativestabtransform_location (`KismetMathLibrary.BreakTransform` (`self.RelativeStabTransform`)))
  (bind _returnvalue (`Actor.GetTransform` (`self.GetOwner`)))
  (bind (_returnvalue_x _returnvalue_y _returnvalue_z) (`KismetMathLibrary.BreakVector` (`KismetMathLibrary.InverseTransformLocation` (`KismetMathLibrary.MakeTransform` (`KismetMathLibrary.TransformLocation` _returnvalue (`self.Offset`)) (.rotation _returnvalue) (.scale _returnvalue)) (`KismetMathLibrary.TransformLocation` (`SceneComponent.GetSocketTransform` (`self.AttachComponent`) (`self.AttachBoneName`) "RTS_World") _relativestabtransform_location))))
  (if (`self.ActiveStabber`)
    ;[1 1 1] Check if Stab Distance is breakable
    (if (> _returnvalue_z (`self.Limit`))
      (`self.DoBreakStabber`))))

(event `DoBreakStabber`
  (bind _physicscomponent (`self.PhysicsComponent`))
  ;[1 1 1] Break Stabber Event
  (`PhysicsConstraintComponent.BreakConstraint` (`self.Physics Constraint`))
  (`PrimitiveComponent.SetSimulatePhysics` _physicscomponent false)
  (`PrimitiveComponent.SetSimulatePhysics` _physicscomponent true)
  (`self.OnStabberBroken` self))

(fn `SetupStabber`
  (params (RootC :type "PrimitiveComponent Object Reference") (PhysicsC :type "PrimitiveComponent Object Reference") (`Hit Result` :type "HitResult Structure") (Constraint :type "PhysicsConstraintComponent Object Reference") (`Stab Limit` :type "Float (double-precision)") (Friction :type "Float (double-precision)") (CenterOffset :type "Vector Structure"))
  (returns (Success :type Boolean))
  (locals (TempLinearVelocity :type "Vector Structure" :default (0.0 0.0 0.0)))
  (bind _physics_constraint (`self.Physics Constraint`))
  (bind _physicsc (`local.PhysicsC`))
  (bind (_hit_result_bblockinghit _hit_result_binitialoverlap _hit_result_time _hit_result_distance _hit_result_location _hit_result_impactpoint _hit_result_normal _hit_result_impactnormal _hit_result_physmat _hit_result_hitactor _hit_result_hitcomponent _hit_result_hitbonename) (`GameplayStatics.BreakHitResult` (`local.Hit Result`)))
  (bind _physics_constraint_2 (`self.Physics Constraint`))
  (bind _physics_constraint_3 (`self.Physics Constraint`))
  (bind (_bblockinghit _binitialoverlap _time _distance _location _impactpoint) (`GameplayStatics.BreakHitResult` (`local.Hit Result`)))
  (bind _returnvalue (`SceneComponent.GetSocketTransform` (`self.AttachComponent`) (`self.AttachBoneName`) "RTS_World"))
  (bind _returnvalue_2 (`KismetMathLibrary.InverseTransformRotation` _returnvalue (.rotation (`SceneComponent.K2_GetComponentToWorld` (`local.PhysicsC`)))))
  (set `self.Physics Constraint` Constraint)
  (set `self.Limit` `Stab Limit`)
  (set `self.Offset` CenterOffset)
  (set `self.AttachComponent` _hit_result_hitcomponent)
  (set `self.AttachBoneName` _hit_result_hitbonename)
  (`|ExecutionSequence`
    (:`then_0`
      (`|ExecutionSequence`
        (:`then_0`
          (`PhysicsConstraintComponent.SetAngularTwistLimit` _physics_constraint_2 "ACM_Locked" 0.0)
          (`PhysicsConstraintComponent.SetAngularSwing1Limit` _physics_constraint_2 "ACM_Locked" 0.0)
          (`PhysicsConstraintComponent.SetAngularSwing2Limit` _physics_constraint_2 "ACM_Locked" 0.0))
        (:`then_1`
          (`PhysicsConstraintComponent.SetLinearXLimit` _physics_constraint_3 "LCM_Locked" 0.0)
          (`PhysicsConstraintComponent.SetLinearYLimit` _physics_constraint_3 "LCM_Locked" 0.0))
        (:`then_2`
          (`PhysicsConstraintComponent.SetLinearZLimit` (`self.Physics Constraint`) "LCM_Limited" (+ (`local.Stab Limit`) 1.0))
          (`PhysicsConstraintComponent.SetDisableCollision` (`self.Physics Constraint`) true)
          (`PhysicsConstraintComponent.SetLinearVelocityDrive` _physics_constraint false false true)
          (`PhysicsConstraintComponent.SetLinearDriveParams` _physics_constraint 0.0 (`local.Friction`) 0.0))))
    (:`then_1`
      ;[1 1 1] Setup Physics Constraint Components and Frames
      (`PhysicsConstraintComponent.SetConstrainedComponents` (`self.Physics Constraint`) (`local.PhysicsC`) "None" (`self.AttachComponent`) (`self.AttachBoneName`))
      (set `self.RelativeStabTransform` (`KismetMathLibrary.MakeTransform` (`KismetMathLibrary.InverseTransformLocation` _returnvalue _impactpoint) _returnvalue_2))
      (`PhysicsConstraintComponent.SetConstraintReferenceFrame` (`self.Physics Constraint`) "Frame2" (`KismetMathLibrary.MakeTransform` (* (`KismetMathLibrary.InverseTransformLocation` _returnvalue (- _impactpoint (`KismetMathLibrary.TransformDirection` (`Actor.GetTransform` (`self.GetOwner`)) (`local.CenterOffset`)))) (.scale _returnvalue)) _returnvalue_2))
      (`PhysicsConstraintComponent.SetConstraintReferenceFrame` (`self.Physics Constraint`) "Frame1" (`KismetMathLibrary.MakeTransform` (0.0 0.0 0.0)))
      (bind _returnvalue_3 (`PrimitiveComponent.GetPhysicsLinearVelocity` (`local.PhysicsC`) "None"))
      (set `local.TempLinearVelocity` _returnvalue_3)
      ;[1 1 1] Reset Physics Simulation to allow Disabled Collision of the Constraints
      (`PrimitiveComponent.SetSimulatePhysics` _physicsc false)
      (`PrimitiveComponent.SetSimulatePhysics` _physicsc true)
      (`PrimitiveComponent.SetAllPhysicsLinearVelocity` (`local.PhysicsC`) (`local.TempLinearVelocity`) false)
      ;[1 1 1] Bind On Destroyed Event of the stabbed Actor
      (add `Actor.OnDestroyed` (`self.GetOwner` (`self.AttachComponent`)) (`|CreateDelegate` :!event `OnAttacherDestroyed`)))
    (:`then_2`
      ;[1 1 1] Setup the Physics Tool itself
      (`self.Setup` (`local.RootC`) (`local.PhysicsC`))
      (return true))))