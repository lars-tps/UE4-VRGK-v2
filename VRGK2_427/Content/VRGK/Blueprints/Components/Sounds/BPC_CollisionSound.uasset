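; Actor component that plays an impact sound when its owner's physics body hits another actor.
; It enables hit notifications on a named primitive or the root, supporting skeletal meshes through closest-bone velocity.
; Hits must pass impulse, relative velocity and direction checks to spawn a sound with impulse-scaled volume and fire OnSoundHit.
; A DoOnce gate with a random reset delay limits sound spam.
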(event `self.ReceiveBeginPlay`
  (bind _primarycomponent (`self.PrimaryComponent`))
  ;[1 1 1] Begin Play
  (add `Actor.OnActorHit` (`self.GetOwner`) (delegate `OnActorHit`))
  (`|ExecutionSequence`
    (:`then_1`
      ;[1 1 1] Setup; Get the Primary Primitive Component to track for hits
      (for _array_element (`Actor.K2_GetComponentsByClass` (`self.GetOwner`) "/Script/Engine.PrimitiveComponent")
        (if (`KismetStringLibrary.EqualEqual_StrStr` (`KismetSystemLibrary.GetObjectName` _array_element) (`self.PrimaryComponentName`))
          (set `self.PrimaryComponent` _array_element)
          (break)))
      (`/Engine/EditorBlueprintResources/StandardMacros.IsValid` (`self.PrimaryComponent`)
        (:`Is Valid`
          (`PrimitiveComponent.SetNotifyRigidBodyCollision` _primarycomponent true :!label _label)
          (bind _asskeletal_mesh_component (cast `SkeletalMeshComponent` _primarycomponent))
          (set `self.PrimarySkeletal` _asskeletal_mesh_component)
          (set `self.IsSkeletal` true))
        (:`Is Not Valid`
          (bind _asprimitive_component (cast `PrimitiveComponent` (`Actor.RootComponent` (`self.GetOwner`)))
            (:`then`
              (set `self.PrimaryComponent` _asprimitive_component)
              (goto _label))
            (:`CastFailed`
              (`KismetSystemLibrary.PrintString` "Sound Collision: No primary Component!" true true (struct :`G` 0.66 :`B` 1.0 :`A` 1.0) 5.0))))))))

(event `OnActorHit`
  (params (SelfActor :type "Actor Object Reference") (OtherActor :type "Actor Object Reference") (NormalImpulse :type "Vector Structure") (Hit :type "HitResult Structure (by ref)"))
  (bind _returnvalue (`KismetMathLibrary.VSize` NormalImpulse))
  (if (!= SelfActor OtherActor)
    (bind _velocity (`self.Calculate Hit Velocity` NormalImpulse Hit))
    ;[1 1 1] Check if Hit is valid for Sound Generation
    (`|ExecutionSequence`
      (:`then_0`
        (if (and (> _returnvalue (`self.ImpactThreshold`)) (> (`KismetMathLibrary.VSize` _velocity) (`self.VelocityThreshold`)) (> (`KismetMathLibrary.Dot_VectorVector` (`KismetMathLibrary.Normal` _velocity) (`KismetMathLibrary.Normal` NormalImpulse)) 0.1))
          ;[1 1 1] Do Once to prevent too many Sounds
          (`/Engine/EditorBlueprintResources/StandardMacros.DoOnce` false :!label _label_2
            (:`Completed`
              ;[1 1 1] Spawn Hit Sound
              (`GameplayStatics.SpawnSoundAtLocation` (`self.HitSound`) (`.ImpactPoint` (`GameplayStatics.BreakHitResult` Hit)) (struct) (* (`KismetMathLibrary.Lerp` (`self.MinVolume`) 1.0 (`KismetMathLibrary.FClamp` (/ (- _returnvalue (`self.ImpactThreshold`)) (`self.VolumeRange`)))) (`self.VolumeMultiplier`)) (`self.PitchMultiplier`) 0.0 (`self.AttenuationOverride`) null)
              (`self.OnSoundHit` Hit)
              ;[1 1 1] Reset after Delay to allow new Sounds from being Spawned
              (`KismetSystemLibrary.Delay` (`KismetMathLibrary.RandomFloatInRange` (`self.HitDelayMin`) (`self.HitDelayMax`)))
              (`self.ResetHitDoOnce`))))))))

(event `ResetHitDoOnce`
  ;[1 1 1] Do Once to prevent too many Sounds
  (goto _label_2 :!via `Reset`))

(fn `Calculate Hit Velocity`
  (params (`Normal Impulse` :type "Vector Structure") (Hit :type "HitResult Structure"))
  (returns (Velocity :type "Vector Structure"))
  (locals (SelfVelocity :type "Vector Structure" :default (0.0 0.0 0.0)) (OtherVelocity :type "Vector Structure" :default (0.0 0.0 0.0)) (HitVelocity :type "Vector Structure" :default (0.0 0.0 0.0)))
  (bind _primaryskeletal (`self.PrimarySkeletal`))
  (bind (_bblockinghit _binitialoverlap _time _distance _location _impactpoint _normal _impactnormal _physmat _hitactor _hitcomponent _hitbonename) (`GameplayStatics.BreakHitResult` (`local.Hit`)))
  (`|ExecutionSequence`
    (:`then_0`
      ;[1 1 1] Calculate Velocity
      (`|ExecutionSequence`
        (:`then_0`
          (`|ExecutionSequence`
            (:`then_0`
              (bind _returnvalue (`PrimitiveComponent.GetPhysicsLinearVelocityAtPoint` _hitcomponent _impactpoint _hitbonename))
              (set `local.OtherVelocity` _returnvalue))
            (:`then_1`
              (if (`self.IsSkeletal`)
                (bind _returnvalue_2 (`PrimitiveComponent.GetPhysicsLinearVelocityAtPoint` _primaryskeletal _impactpoint (`.ReturnValue` (`SkinnedMeshComponent.FindClosestBone_K2` _primaryskeletal _impactpoint 0.0 false))))
                (set `local.SelfVelocity` _returnvalue_2)
                (else
                  (bind _returnvalue_3 (`PrimitiveComponent.GetPhysicsLinearVelocityAtPoint` (`self.PrimaryComponent`) _impactpoint "None"))
                  (set `local.SelfVelocity` _returnvalue_3))))))
        (:`then_1`
          (if (`SceneComponent.IsSimulatingPhysics` _hitcomponent _hitbonename)
            (set `local.HitVelocity` (- (`local.SelfVelocity`) (`local.OtherVelocity`)))
            (else
              (set `local.HitVelocity` (`local.SelfVelocity`)))))))
    (:`then_1`
      (`|ExecutionSequence`
        (:`then_1`
          (return (`local.HitVelocity`)))))))