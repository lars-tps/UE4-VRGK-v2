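; Actor component for the VR base pawn that plays a movement wind sound which responds to the pawn's speed.
; On BeginPlay it attaches a silent, low-pitched looping-style audio component to the pawn's camera.
; Each tick it maps velocity length to volume and pitch targets within a speed range.
; Both values interpolate toward those targets, with separate rates for speeding up and slowing down.
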(event `self.ReceiveBeginPlay`
  (bind _asbp_vrbase_pawn (cast `/Game/VRGK/Blueprints/Player/PlayerCore/BP_VRBasePawn` (`self.GetOwner`)))
  (bind _output_get (set `self.VRPawn` _asbp_vrbase_pawn))
  (bind _returnvalue (`GameplayStatics.SpawnSoundAttached` (`self.Movement Sound`) (`/Game/VRGK/Blueprints/Player/PlayerCore/BP_VRBasePawn.Camera` _output_get) "None" (0.0 0.0 0.0) (struct) "SnapToTarget" false 0.0 0.5 0.0 null null false))
  (set `self.AudioComponent` _returnvalue))

(event `self.ReceiveTick`
  (params (DeltaSeconds :type "Float (single-precision)"))
  (bind _audiocomponent (`self.AudioComponent`))
  (bind _audiocomponent_2 (`self.AudioComponent`))
  (set `self.TempVelocity` (`KismetMathLibrary.VSize` (`Actor.GetVelocity` (`self.VRPawn`))))
  (set `self.Increasing` (> (`self.TempVelocity`) (`self.LastVelocity`)))
  (set `self.LastVelocity` (`self.TempVelocity`))
  (`|ExecutionSequence`
    (:`then_0`
      (`AudioComponent.SetVolumeMultiplier` _audiocomponent_2 (`KismetMathLibrary.FInterpTo` (`AudioComponent.VolumeMultiplier` _audiocomponent_2) (`KismetMathLibrary.MapRangeClamped` (`self.TempVelocity`) (`self.Velocity Min`) (`self.Velocity Max`) 0.0 1.0) DeltaSeconds (`KismetMathLibrary.SelectFloat` (`self.VolumeInterpSpeedUp`) (`self.VolumeInterpSpeedDown`) (`self.Increasing`)))))
    (:`then_1`
      (`AudioComponent.SetPitchMultiplier` _audiocomponent (`KismetMathLibrary.FInterpTo` (`AudioComponent.PitchMultiplier` _audiocomponent) (`KismetMathLibrary.MapRangeClamped` (`self.TempVelocity`) (`self.Velocity Min`) (`self.Velocity Max`) 0.5 2.0) DeltaSeconds (`KismetMathLibrary.SelectFloat` (`self.PitchInterpSpeedUp`) (`self.PitchInterpSpeedDown`) (`self.Increasing`)))))))