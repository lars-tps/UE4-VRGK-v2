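; BP_PlayerInventoryBag is an inventory bag actor that follows the body of the VR player pawn.
; On BeginPlay it casts its owner to BP_VRGamePawn, caches it, and destroys itself when that pawn ends play.
; Every Tick it moves to the pawn's camera location, taking rotation from CalculateBodyWorldRotation rather than the camera.
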(event `self.ReceiveBeginPlay`
  (bind _asbp_vrgame_pawn (cast `/Game/VRGK/Blueprints/Player/PlayerCore/BP_VRGamePawn` (`self.GetOwner`)))
  (bind _output_get (set `self.VRPawn` _asbp_vrgame_pawn))
  (add `self.OnEndPlay` _output_get (delegate `OnPlayerEndPlay`)))

(event `OnPlayerEndPlay` :!signature `self.OnEndPlay`
  (params (Actor :type "Actor Object Reference") (EndPlayReason :type "EEndPlayReason Enum" :default "Destroyed"))
  (`self.K2_DestroyActor`))

(event `self.ReceiveTick`
  (params (DeltaSeconds :type "Float (single-precision)"))
  (bind _vrpawn (`self.VRPawn`))
  (bind _returnvalue_location (`KismetMathLibrary.BreakTransform` (`SceneComponent.K2_GetComponentToWorld` (`/Game/VRGK/Blueprints/Player/PlayerCore/BP_VRBasePawn.Camera` _vrpawn))))
  (`self.K2_SetActorLocationAndRotation` _returnvalue_location (`/Game/VRGK/Blueprints/Player/PlayerCore/BP_VRBasePawn.Calculate Body World Rotation` _vrpawn)))

(fn `UserConstructionScript`)