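; Base actor for a VR inventory slot that holds one actor carrying a BPC_VRInventoryItem component.
; Storing requires an empty slot, a tag match and the item's consent; store and drop both delegate to that component and play a sound.
; An empty tag list accepts any item not restricted to tagged slots, and an optional dot-product check validates grab direction.
; When its parent actor ends play, the slot drops its item and destroys itself.
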(event `self.ReceiveBeginPlay`
  (add `self.OnEndPlay` (`self.GetParentActor`) (delegate `OnParentEndPlay`)))

(event `OnParentEndPlay` :!signature `self.OnEndPlay`
  (params (Actor :type "Actor Object Reference") (EndPlayReason :type "EEndPlayReason Enum" :default "Destroyed"))
  (`self.DropActor`)
  (`self.K2_DestroyActor`))

(fn `Check Item Compatibility`
  (params (ItemActor :type "Actor Object Reference"))
  (returns (Compatible :type Boolean))
  (bind (_valid _inventoryitem) (`self.GetInventoryItem` ItemActor))
  (bind _alloweditemtags (`self.AllowedItemTags`))
  (bind _returnvalue (`KismetArrayLibrary.Array_Contains` _alloweditemtags (`/Game/VRGK/Blueprints/Inventory/BPC_VRInventoryItem.ItemTag` _inventoryitem)))
  (`/Engine/EditorBlueprintResources/StandardMacros.IsValid` ItemActor
    (:`Is Valid`
      (if _valid
        (return (select `bool` (`/Game/VRGK/Blueprints/Inventory/BPC_VRInventoryItem.OnlyAllowStoringWithTag` _inventoryitem) :`false` (or (<= (`KismetArrayLibrary.Array_Length` _alloweditemtags) 0) _returnvalue) :`true` _returnvalue))
        (else
          _)))
    (:`Is Not Valid`
      _))
  (return false))

(fn `CheckForValidDirection`
  (params (GrabWorldLocation :type "Vector Structure") (GrabForwardVector :type "Vector Structure"))
  (returns (`Valid Direction` :type Boolean))
  (return (select `bool` (`self.OnlyGrabWhenLookingAtSlot`) :`false` true :`true` (> (`KismetMathLibrary.Dot_VectorVector` (`KismetMathLibrary.Normal` (- (`self.K2_GetActorLocation`) GrabWorldLocation)) GrabForwardVector) 0.0))))

(fn `DropActor`
  (returns (Valid :type Boolean) (DroppedActor :type "Actor Object Reference"))
  (locals (ActorToDrop :type "Actor Object Reference"))
  (bind _storedactor (`self.GetStoredActor`))
  (if (`self.IsStoringActor`)
    (set `local.ActorToDrop` _storedactor)
    (`/Game/VRGK/Blueprints/Inventory/BPC_VRInventoryItem.Drop  From Inventory Slot` (`.InventoryItem` (`self.GetInventoryItem` _storedactor)))
    (set `self.StoredActor` null)
    (`|ExecutionSequence`
      (:`then_0`
        (`GameplayStatics.SpawnSoundAttached` (`self.DropSound`) (`self.DefaultSceneRoot`) "None" (0.0 0.0 0.0) (struct) "SnapToTarget" false 1.0 1.0 0.0 null null))
      (:`then_1`
        (return true (`local.ActorToDrop`))))
    (else
      (return false null))))

(fn `GetInventoryItem`
  (params (Actor :type "Actor Object Reference"))
  (returns (Valid :type Boolean) (InventoryItem :type "/Game/VRGK/Blueprints/Inventory/BPC_VRInventoryItem Object Reference"))
  (bind _returnvalue (`self.GetComponentByClass` Actor "/Game/VRGK/Blueprints/Inventory/BPC_VRInventoryItem.BPC_VRInventoryItem_C"))
  (return (`KismetSystemLibrary.IsValid` _returnvalue) _returnvalue))

(fn `GetStoredActor`
  (returns (StoredActor :type "Actor Object Reference"))
  (return (`self.StoredActor`)))

(fn `IsStoringActor`
  (returns (ReturnValue :type Boolean))
  (return (`KismetSystemLibrary.IsValid` (`self.GetStoredActor`))))

(fn `StoreActor`
  (params (Actor :type "Actor Object Reference"))
  (returns (Successful :type Boolean))
  (bind (_valid _inventoryitem) (`self.GetInventoryItem` Actor))
  (`/Engine/EditorBlueprintResources/StandardMacros.IsValid` Actor
    (:`Is Valid`
      (if (`self.IsStoringActor`)
        (return false)
        (elif _valid
          (bind _compatible (`self.Check Item Compatibility` Actor))
          (if _compatible
            (if (`/Game/VRGK/Blueprints/Inventory/BPC_VRInventoryItem.CanBeStored` _inventoryitem)
              (bind _output_get (set `self.StoredActor` Actor))
              (`/Game/VRGK/Blueprints/Inventory/BPC_VRInventoryItem.Store In Inventory Slot` (`.InventoryItem` (`self.GetInventoryItem` _output_get)) self)
              (`|ExecutionSequence`
                (:`then_0`
                  (`GameplayStatics.SpawnSoundAttached` (`self.StoreSound`) (`self.DefaultSceneRoot`) "None" (0.0 0.0 0.0) (struct) "SnapToTarget" false 1.0 1.0 0.0 null null))
                (:`then_1`
                  (return true)))
              (else
                (return false)))
            (else
              (return false)))
          (else
            (return false)))))
    (:`Is Not Valid`
      (return false))))

(fn `UserConstructionScript`)