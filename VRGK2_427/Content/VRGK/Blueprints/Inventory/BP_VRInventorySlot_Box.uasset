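; Box-shaped VR inventory slot that adds its setup on top of a parent class.
; UpdateBoxPosition applies the BoxExtent and BoxTransform variables to the Box component's size and relative transform.
; It runs from the construction script and again on BeginPlay, each time after the parent's logic.
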(event `self.ReceiveBeginPlay`
  (`parent.ReceiveBeginPlay`)
  (`self.UpdateBoxPosition`))

(event `UpdateBoxPosition`
  (bind _box (`self.Box`))
  (`BoxComponent.SetBoxExtent` _box (`self.BoxExtent`) true)
  (`SceneComponent.K2_SetRelativeTransform` _box (`self.BoxTransform`) false false))

(fn `UserConstructionScript`
  (`parent.UserConstructionScript`)
  (`self.UpdateBoxPosition`))