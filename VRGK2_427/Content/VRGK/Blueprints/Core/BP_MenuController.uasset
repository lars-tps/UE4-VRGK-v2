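; BP_MenuController runs the VR pause menu, pausing the game and swapping between the player pawn and a temporary menu pawn.
; Opening spawns and possesses BP_VRMenuPawn and places BP_MenuOverlay at the camera.
; A pause-tickable timeline fades the world through MPC_Global's "Pause" parameter.
; Closing reverses this and offsets the VR origin by horizontal head movement, preventing walking through walls while in the menu.
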(event `self.ReceiveBeginPlay`
  (`ActorComponent.SetTickableWhenPaused` (`self.PauseFadeTimeline`) true))

(event `SetPaused`
  (params (Paused :type Boolean))
  ;[1 1 1] SetPaused
  (if Paused
    (`GameplayStatics.SetGamePaused` true)
    (set `self.IsPaused` true)
    (else
      (`GameplayStatics.SetGamePaused` false)
      (set `self.IsPaused` false))))

(event `OpenMenu`
  (params (FromPawn :type "/Game/VRGK/Blueprints/Player/PlayerCore/BP_VRBasePawn Object Reference"))
  (bind _playerpawn (`self.PlayerPawn`))
  (bind _playerpawn_2 (`self.PlayerPawn`))
  (bind _camera (`/Game/VRGK/Blueprints/Player/PlayerCore/BP_VRBasePawn.Camera` _playerpawn))
  (bind (_forward_vector _right_vector) (`/Game/VRGK/Blueprints/Player/PlayerCore/BP_VRBasePawn.Calculate VRVectors` _playerpawn _camera))
  ;[1 1 1] OpenMenu and spawn MenuPawn
  (set `self.PlayerPawn` FromPawn)
  (`self.SetPaused` true)
  (bind _returnvalue (`|SpawnActorFromClass` "/Game/VRGK/Blueprints/Player/Menu/BP_VRMenuPawn.BP_VRMenuPawn_C" (`self.GetTransform` _playerpawn_2) "AlwaysSpawn" "OverrideRootScale" null _playerpawn_2 "NewEnumerator0" null))
  (bind _output_get (set `self.MenuPawn` _returnvalue))
  (`Controller.Possess` (`GameplayStatics.GetPlayerController` 0) _output_get)
  (`/Game/VRGK/Blueprints/Player/PlayerCore/BP_VRBasePawn.MenuOpened` (`self.PlayerPawn`))
  (bind _returnvalue_2 (`|SpawnActorFromClass` "/Game/VRGK/Blueprints/Menu/BP_MenuOverlay.BP_MenuOverlay_C" (`KismetMathLibrary.MakeTransform` (`SceneComponent.K2_GetComponentLocation` _camera) (`KismetMathLibrary.MakeRotFromXY` _forward_vector _right_vector)) "Undefined" "OverrideRootScale" null null))
  (set `self.MenuOverlay` _returnvalue_2)
  ;[1 1 1] Update Post Process World Fade Effect
  (bind (_direction _worldfadealpha) (`Timeline|PauseFadeTimeline` :!label _label)
    (:`Update`
      _)
    (:`Finished`
      _))
  (`KismetMaterialLibrary.SetScalarParameterValue` "/Game/VRGK/Materials/PostProcess/MPC_Global.MPC_Global" "Pause" _worldfadealpha))

(event `CloseMenu`
  (bind (_returnvalue_x _returnvalue_y) (`KismetMathLibrary.BreakVector` (- (`SceneComponent.RelativeLocation` (`/Game/VRGK/Blueprints/Player/PlayerCore/BP_VRBasePawn.Camera` (`self.PlayerPawn`))) (`SceneComponent.RelativeLocation` (`/Game/VRGK/Blueprints/Player/PlayerCore/BP_VRBasePawn.Camera` (`self.MenuPawn`))))))
  ;[1 1 1] Close Menu and return to GamePawn
  ;;[1 0.2583 0.2682] Reset IRL Player Position to Game Player Position. Stops walking through walls in the menu.
  (`SceneComponent.K2_AddLocalOffset` (`/Game/VRGK/Blueprints/Player/PlayerCore/BP_VRBasePawn.VROriginRoot` (`self.PlayerPawn`)) (`KismetMathLibrary.MakeVector` _returnvalue_x _returnvalue_y) false false)
  (`self.SetPaused` false)
  (`Controller.Possess` (`GameplayStatics.GetPlayerController` 0) (`self.PlayerPawn`))
  (`self.K2_DestroyActor` (`self.MenuPawn`))
  (`/Game/VRGK/Blueprints/Player/PlayerCore/BP_VRBasePawn.MenuClosed` (`self.PlayerPawn`))
  (`self.K2_DestroyActor` (`self.MenuOverlay`))
  (set `self.MenuOverlay` null)
  (goto _label :!via `Reverse`))

(fn `UserConstructionScript`)